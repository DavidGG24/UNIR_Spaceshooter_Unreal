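; Player pawn for the space shooter, moved through Enhanced Input.
; BeginPlay adds the IMC_Player mapping context to the controlling player's input subsystem.
; The movement action stores a 2D input, zeroed on release or cancel, which Tick scales by Speed and delta time along right and forward vectors.
; Movement sets location directly without sweeping, and the fire action only prints a debug string.
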(event Input|EnhancedActionEvents|EnhancedInputActionIA_Player_Fire
  (params (ActionValue :type Boolean) (ElapsedSeconds :type Float%20%28double-precision%29) (TriggeredSeconds :type Float%20%28double-precision%29) (InputAction :type Input%20Action%20Object%20Reference :default "/Game/SpaceShooter/Input/IA_Player_Fire.IA_Player_Fire"))
  (:Triggered
    (Development|PrintString "Fired")))

(event Input|EnhancedActionEvents|EnhancedInputActionIA_Player_Movement
  (params (ActionValue :type Vector%202D%20Structure) (ElapsedSeconds :type Float%20%28double-precision%29) (TriggeredSeconds :type Float%20%28double-precision%29) (InputAction :type Input%20Action%20Object%20Reference :default "/Game/SpaceShooter/Input/IA_Player_Movement.IA_Player_Movement"))
  (:Triggered
    (Variables|Default|SetMovementInput ActionValue))
  (:Canceled
    (Variables|Default|SetMovementInput "" :!label _label))
  (:Completed
    (goto _label)))

(event EventBeginPlay
  (bind _asplayer_controller (Utilities|Casting|CastToPlayerController (Pawn|GetController)))
  (Utilities|IsValid (PlayerController|LocalPlayerSubsystems|GetEnhancedInputLocalPlayerSubsystem _asplayer_controller)
    (:Is%20Valid
      (Input|AddMappingContext (PlayerController|LocalPlayerSubsystems|GetEnhancedInputLocalPlayerSubsystem _asplayer_controller) "/Game/SpaceShooter/Input/IMC_Player.IMC_Player" 0 "(bIgnoreAllPressedKeysUntilRelease=True,bForceImmediately=False,bNotifyUserSettings=False)"))))

(event Collision|EventActorBeginOverlap
  (params (OtherActor :type Actor%20Object%20Reference)))

(event EventTick
  (params (DeltaSeconds :type Float%20%28single-precision%29))
  (bind _speed (Variables|Default|GetSpeed))
  (bind _movementinput (Variables|Default|GetMovementInput))
  (bind _returnvalue (* DeltaSeconds _speed))
  (Transformation|SetActorLocation (+ (+ (* (Transformation|GetActorRightVector) (* _returnvalue (.x _movementinput))) (* (* _returnvalue (.y _movementinput)) (Transformation|GetActorForwardVector))) (Transformation|GetActorLocation)) false false))

(fn ConstructionScript)