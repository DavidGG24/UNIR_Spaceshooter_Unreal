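; BP_Enemy_Base is the base enemy actor for a space shooter: it flies straight, fires on a timer and dies on contact with the player.
; Tick moves it along the forward vector cached at BeginPlay and accumulates time to spawn Ammo at FirePoint, aligned to its rotation.
; Overlapping a Player-tagged actor calls the OnEnemyDestroy dispatcher, whose self-bound handler destroys the enemy after a short delay.
; An ammo cast leading to that dispatcher is left unconnected.
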(event Custom|DestroyedEvent
  (Utilities|FlowControl|Delay 0.1)
  (Actor|DestroyActor))

(event EventBeginPlay
  (Variables|Default|SetMovementVector (Transformation|GetActorForwardVector))
  (EventDispatchers|BindEventtoOnEnemyDestroy (delegate Custom|DestroyedEvent)))

(event Collision|EventActorBeginOverlap
  (params (OtherActor :type Actor%20Object%20Reference))
  (if (Utilities|Array|ContainsItem (Variables|/Script/Engine.Actor|GetTags OtherActor) "Player")
    (Default|CallOnEnemyDestroy)))

(event EventTick
  (params (DeltaSeconds :type Float%20%28single-precision%29))
  (CallFunction|Move DeltaSeconds)
  (bind _output_get (Variables|Default|SetShootCurrentTIme (+ DeltaSeconds (Variables|Default|GetShootCurrentTIme))))
  (if (> _output_get (Variables|Default|GetDelayShoot))
    (Variables|Default|SetShootCurrentTIme 0.0)
    (CallFunction|Fire)))

(fn ConstructionScript)

(fn Move
  (params (DeltaSeconds :type Float%20%28double-precision%29))
  (Transformation|SetActorLocation (+ (Transformation|GetActorLocation) (* (* DeltaSeconds (Variables|Default|GetSpeed)) (Variables|Default|GetMovementVector))) false false))

(fn Fire
  (bind _returnvalue (Game|SpawnActorfromClass (Variables|Default|GetAmmo) (Transformation|GetWorldTransform (Variables|Default|GetFirePoint)) "Undefined" "MultiplyWithRoot" 0 0))
  (Transformation|SetActorRotation _returnvalue (Transformation|GetActorRotation)))