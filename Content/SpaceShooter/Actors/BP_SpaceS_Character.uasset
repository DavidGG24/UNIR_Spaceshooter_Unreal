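; Player character for the Space Shooter game, handling movement, firing and lives.
; On BeginPlay it adds the Enhanced Input mapping context, then input drives movement along the actor's right and forward vectors.
; Firing spawns the Ammo class at SpawnPoint, with a CanFire flag and timer enforcing the delay between shots.
; DamageActor removes a life and notifies the SSGamemode of player death when lives reach zero.
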(event Custom|ResetCanFire
  (Variables|Default|SetCanFire true))

(event Custom|DamageActor
  (bind _output_get (Variables|Default|SetLifes (- (Variables|Default|GetLifes) 1)))
  (if (== _output_get 0)
    (bind _asssgamemode (Utilities|Casting|CastToSSGamemode (Game|GetGameMode)))
    (Default|PlayerDeath _asssgamemode)))

(event Input|EnhancedActionEvents|EnhancedInputActionIA_Player_Movement
  (params (ActionValue :type Vector%202D%20Structure) (ElapsedSeconds :type Float%20%28double-precision%29) (TriggeredSeconds :type Float%20%28double-precision%29) (InputAction :type Input%20Action%20Object%20Reference :default "/Game/SpaceShooter/Input/IA_Player_Movement.IA_Player_Movement"))
  (:Triggered
    (Pawn|Input|AddMovementInput (Transformation|GetActorRightVector) (.x ActionValue) false)
    (Pawn|Input|AddMovementInput (Transformation|GetActorForwardVector) (.y ActionValue) false)))

(event Input|EnhancedActionEvents|EnhancedInputActionIA_Player_Fire
  (params (ActionValue :type Boolean) (ElapsedSeconds :type Float%20%28double-precision%29) (TriggeredSeconds :type Float%20%28double-precision%29) (InputAction :type Input%20Action%20Object%20Reference :default "/Game/SpaceShooter/Input/IA_Player_Fire.IA_Player_Fire"))
  (:Triggered
    (if (Variables|Default|GetCanFire)
      (CallFunction|DoFire)
      (Variables|Default|SetCanFire false)
      (Utilities|Time|SetTimerbyEvent (delegate Custom|ResetCanFire) (Variables|Default|GetFireDelay)))))

(event EventBeginPlay
  (bind _asplayer_controller (Utilities|Casting|CastToPlayerController (Pawn|GetController)))
  (Utilities|IsValid (PlayerController|LocalPlayerSubsystems|GetEnhancedInputLocalPlayerSubsystem _asplayer_controller)
    (:Is%20Valid
      (Input|AddMappingContext (PlayerController|LocalPlayerSubsystems|GetEnhancedInputLocalPlayerSubsystem _asplayer_controller) "/Game/SpaceShooter/Input/IMC_Player.IMC_Player" 0 "(bIgnoreAllPressedKeysUntilRelease=True,bForceImmediately=False,bNotifyUserSettings=False)"))))

(event Collision|EventActorBeginOverlap
  (params (OtherActor :type Actor%20Object%20Reference)))

(event EventTick
  (params (DeltaSeconds :type Float%20%28single-precision%29)))

(fn ConstructionScript)

(fn DoFire
  (Game|SpawnActorfromClass (Variables|Default|GetAmmo) (Transformation|GetWorldTransform (Variables|Default|GetSpawnPoint)) "Undefined" "MultiplyWithRoot" 0 0))