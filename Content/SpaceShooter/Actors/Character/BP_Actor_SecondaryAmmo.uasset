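; BP_Actor_SecondaryAmmo is the space shooter's secondary projectile, which explodes on overlap or after traveling a set distance along X.
; It swaps Capsule collision for Explosion collision to create a blast area, deferring other overlap and movement behavior to its parent.
; Tick compares X against the spawn position and, once past range, spawns explosion effects and sound, then briefly delays before destroying the actor.
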(event EventBeginPlay
  (|CallParentFunction)
  (Collision|SetCollisionEnabled (Variables|Default|GetExplosion) "NoCollision")
  (Variables|Default|SetBulletStartPos (Transformation|GetActorLocation)))

(event Collision|EventActorBeginOverlap
  (params (OtherActor :type Actor%20Object%20Reference))
  (Collision|SetCollisionEnabled (Variables|Default|GetCapsule) "NoCollision")
  (Collision|SetCollisionEnabled (Variables|Default|GetExplosion) "QueryAndPhysics")
  (|CallParentFunction OtherActor))

(event EventTick
  (params (DeltaSeconds :type Float%20%28single-precision%29))
  (|CallParentFunction DeltaSeconds)
  (if (and (> (- (.x (Transformation|GetActorLocation)) (.x (Variables|Default|GetBulletStartPos))) 3.8e+02) (== (Variables|Default|GetExploded) false))
    (Variables|Default|SetExploded true)
    (Collision|SetCollisionEnabled (Variables|Default|GetCapsule) "NoCollision")
    (Collision|SetCollisionEnabled (Variables|Default|GetExplosion) "QueryAndPhysics")
    (Effects|SpawnEmitteratLocation "/Game/StarterContent/Particles/P_Explosion.P_Explosion" (Transformation|GetActorLocation))
    (Audio|PlaySound2D "/Game/StarterContent/Audio/Explosion02.Explosion02" 1.0 1.0 0.0 0 0)
    (Utilities|FlowControl|Delay 0.1)
    (Actor|DestroyActor)))

(fn ConstructionScript
  (|CallParentFunction))